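; BP_ItemInventario is an inventory pickup actor that can be collected from the world.
; PickupItem returns its Itemstring, while Recogeritem returns its ItemInventario data, labelled as a struct in its debug print.
; Both print a debug message and call Destruir, which waits one tick before destroying the actor.
; The Interactuar event is present but has no logic.
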(event Custom|destruir
  (Utilities|FlowControl|DelayUntilNextTick)
  (Actor|DestroyActor))

(event EventBeginPlay)

(event Collision|EventActorBeginOverlap
  (params (OtherActor :type Actor%20Object%20Reference)))

(event EventTick
  (params (DeltaSeconds :type Float%20%28single-precision%29)))

(event EventInteractuar
  (params (character :type BP%20Character%20Object%20Reference)))

(fn ConstructionScript)

(fn PickupItem
  (Development|PrintString "recogi un objeto")
  (CallFunction|Destruir)
  (return (Variables|Default|Getitemstring)))

(fn Recogeritem
  (Development|PrintString "recogiendo objeto con struct")
  (CallFunction|Destruir)
  (return (Variables|Default|GetItemInventario)))