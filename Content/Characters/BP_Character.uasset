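; Player character Blueprint with Enhanced Input movement (sprint, jump, dash), melee combos, shooting, weapon pickup and quest interaction.
; Health and experience components broadcast changes that update the WBP_ui HUD.
; Dash line-traces to snap to a hit point or launches forward, with gravity and capsule collision temporarily off.
; Melee chains montages with a kick gated by level, HitDetect sphere-traces limb sockets, and shooting spawns projectiles on montage notifies.
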(event Custom|salud%20inicial
  (params (Vida :type Float%20%28double-precision%29) (Vida%20max :type Float%20%28double-precision%29))
  (Default|Actualizarvida (Variables|Default|Getui) Vida Vida%20max))

(event Custom|Dano%20recibido
  (params (Vida :type Float%20%28double-precision%29) (Vida%20max :type Float%20%28double-precision%29))
  (Default|Actualizarvida (Variables|Default|Getui) Vida Vida%20max))

(event Custom|Dis
  (Variables|/Script/Engine.CharacterMovementComponent|SetGravityScale (Variables|Character|GetCharacterMovement) 1.0)
  (Collision|SetCollisionEnabled (Variables|Default|GetCapsuleComponent) "QueryAndPhysics")
  (Utilities|Time|ClearTimerbyFunctionName 0 "DashCompletado"))

(event Custom|SumoExperiencia
  (params (XP :type Float%20%28double-precision%29) (XP%20Max :type Float%20%28double-precision%29))
  (Default|ActualizarEXP (Variables|Default|Getui) XP XP%20Max))

(event Custom|SumoLevel
  (params (nivel :type Integer))
  (Default|ActualizarLVL (Variables|Default|Getui) nivel))

(event Custom|CuracionRecibida
  (params (Vida :type Float%20%28double-precision%29) (VidaMax :type Float%20%28double-precision%29))
  (Default|Actualizarvida (Variables|Default|Getui) Vida VidaMax))

(event Custom|ExperienciaAlEmpezar
  (params (XP :type Float%20%28double-precision%29) (XPMax :type Float%20%28double-precision%29))
  (Default|ActualizarEXP (Variables|Default|Getui) XP XPMax))

(event Custom|levelinicial
  (params (level :type Integer))
  (Default|ActualizarLVL (Variables|Default|Getui) level))

(event Custom|SpawndeArmas
  (params (spawnarma :type BP%20Armas%20Master%20Class%20Reference))
  (bind _mesh (Variables|Character|GetMesh))
  ;[0.15 0.15 0.15 0.5] Sistema de armas
  ;;[0.15 0.15 0.15 0.5] tirar arma
  (Utilities|IsValid (Variables|Default|GetArmaActual)
    (:Is%20Valid
      (Game|SpawnActorfromClass (Variables|/Game/pickups/BP_ArmasMaster.BP_ArmasMaster_C|GetPickupClass (Variables|Default|GetArmaActual)) (Math|Transform|MakeTransform (+ (Transformation|GetActorLocation) (* (Transformation|GetActorForwardVector) "200.000000,200.000000,0.000000")) "0, 0, 0" "1.000000,1.000000,1.000000") "Undefined" "MultiplyWithRoot" 0 0)
      (Actor|DestroyActor (Variables|Default|GetArmaActual)))
    (:Is%20Not%20Valid
      _))
  ;;[0.15 0.15 0.15 0.5] spawn nueva arma
  (bind _returnvalue (Game|SpawnActorfromClass spawnarma (Math|Transform|MakeTransform (Transformation|GetActorLocation) "0, 0, 0" "1.000000,1.000000,1.000000") "Undefined" "MultiplyWithRoot" 0 0))
  (bind _output_get (Variables|Default|SetArmaActual _returnvalue))
  (switch Utilities|FlowControl|Switch|SwitchonEnum_NombreEquipo (Variables|/Game/pickups/BP_ArmasMaster.BP_ArmasMaster_C|GetArmaNombre _output_get)
    (:NewEnumerator1
      (Transformation|AttachComponentToComponent _output_get _mesh "SocketPick" "SnapToTarget" "SnapToTarget" "SnapToTarget" true))
    (:NewEnumerator3
      (Transformation|AttachComponentToComponent _output_get _mesh "PistolaSocket" "SnapToTarget" "SnapToTarget" "SnapToTarget" true))
    (:NewEnumerator4
      (Transformation|AttachComponentToComponent _output_get _mesh "SocketEspada" "SnapToTarget" "SnapToTarget" "SnapToTarget" true)
      (Variables|Default|SetTengoUnArmaMele true))))

(event Custom|DashCompletado
  ;[0.15 0.15 0.15 0.5] dash
  (Variables|/Script/Engine.CharacterMovementComponent|SetGravityScale (Variables|Character|GetCharacterMovement) 1.0)
  (Collision|SetCollisionEnabled (Variables|Default|GetCapsuleComponent) "QueryAndPhysics")
  (Utilities|Time|ClearTimerbyFunctionName 0 "DashCompletado"))

(event Input|EnhancedActionEvents|EnhancedInputActionIA_Inventario
  (params (ActionValue :type Boolean) (ElapsedSeconds :type Float%20%28double-precision%29) (TriggeredSeconds :type Float%20%28double-precision%29) (InputAction :type Input%20Action%20Object%20Reference :default "/Game/imputs/IA_Inventario.IA_Inventario")))

(event Input|EnhancedActionEvents|EnhancedInputActionIA_Salto
  (params (ActionValue :type Boolean) (ElapsedSeconds :type Float%20%28double-precision%29) (TriggeredSeconds :type Float%20%28double-precision%29) (InputAction :type Input%20Action%20Object%20Reference :default "/Game/imputs/IA_Salto.IA_Salto"))
  (bind _springarm (Variables|Default|GetSpringArm))
  ;[0.15 0.15 0.15 0.5] salto
  (:Started
    (Character|Jump)
    (Variables|/Script/Engine.SpringArmComponent|SetTargetArmLength _springarm 9e+02))
  (:Completed
    (Character|StopJumping)
    (Utilities|FlowControl|Delay 0.7)
    (Variables|/Script/Engine.SpringArmComponent|SetTargetArmLength _springarm 7.5e+02)))

(event Input|EnhancedActionEvents|EnhancedInputActionIA_Dash
  (params (ActionValue :type Boolean) (ElapsedSeconds :type Float%20%28double-precision%29) (TriggeredSeconds :type Float%20%28double-precision%29) (InputAction :type Input%20Action%20Object%20Reference :default "/Game/imputs/IA_Dash.IA_Dash"))
  (bind _returnvalue (Transformation|GetActorLocation))
  (bind _returnvalue_2 (Transformation|GetActorForwardVector))
  (bind _velocidaddash (Variables|Default|GetVelocidadDash))
  (bind _returnvalue_3 (* _returnvalue_2 _velocidaddash))
  ;[0.15 0.15 0.15 0.5] dash
  (:Started
    (if (not (AI|Components|NavMovement|IsFalling (Variables|Character|GetCharacterMovement)))
      (if (not (Variables|Default|GetDashAcrtivado?))
        (Variables|Default|SetDashAcrtivado? true)
        (Collision|SetCollisionEnabled (Variables|Default|GetCapsuleComponent) "NoCollision")
        (Variables|/Script/Engine.CharacterMovementComponent|SetGravityScale (Variables|Character|GetCharacterMovement) 0.0)
        (bind (_outhit _returnvalue_4) (Collision|LineTraceForObjects _returnvalue (+ _returnvalue (Math|Vector|MakeVector (.x _returnvalue_3) (.y _returnvalue_3) 0.0)) (Utilities|Array|MakeArray "ObjectTypeQuery1" "ObjectTypeQuery2") false 0 "None"))
        (if _returnvalue_4
          (Transformation|SetActorLocation (.ImpactPoint (Collision|BreakHitResult _outhit)) (.bBlockingHit (Collision|BreakHitResult _outhit)) false)
          (else
            (Character|LaunchCharacter (* (Transformation|GetActorForwardVector) (Variables|Default|GetVelocidadDash)) true false)))
        (Utilities|Time|SetTimerbyEvent (delegate Custom|DashCompletado) (Variables|Default|GetDuracionDash))
        (Utilities|FlowControl|Delay (Variables|Default|GetTiempoRecargaDash))
        (Variables|Default|SetDashAcrtivado? false)))))

(event Input|EnhancedActionEvents|EnhancedInputActionIA_Mirar
  (params (ActionValue :type Vector%202D%20Structure) (ElapsedSeconds :type Float%20%28double-precision%29) (TriggeredSeconds :type Float%20%28double-precision%29) (InputAction :type Input%20Action%20Object%20Reference :default "/Game/imputs/IA_Mirar.IA_Mirar")))

(event Input|EnhancedActionEvents|EnhancedInputActionIA_Correr
  (params (ActionValue :type Boolean) (ElapsedSeconds :type Float%20%28double-precision%29) (TriggeredSeconds :type Float%20%28double-precision%29) (InputAction :type Input%20Action%20Object%20Reference :default "/Game/imputs/IA_Correr.IA_Correr"))
  (bind _charactermovement (Variables|Character|GetCharacterMovement))
  ;[0.15 0.15 0.15 0.5] correr
  (:Started
    (Variables|/Script/Engine.CharacterMovementComponent|SetMaxWalkSpeed _charactermovement (* (Variables|/Script/Engine.CharacterMovementComponent|GetMaxWalkSpeed _charactermovement) 3.0)))
  (:Completed
    (Variables|/Script/Engine.CharacterMovementComponent|SetMaxWalkSpeed _charactermovement 4e+02)))

(event Input|EnhancedActionEvents|EnhancedInputActionIA_AtaqueMele
  (params (ActionValue :type Boolean) (ElapsedSeconds :type Float%20%28double-precision%29) (TriggeredSeconds :type Float%20%28double-precision%29) (InputAction :type Input%20Action%20Object%20Reference :default "/Game/imputs/IA_AtaqueMele.IA_AtaqueMele"))
  ;[0.15 0.15 0.15 0.5] ataque mele
  (if (not (Variables|Default|GetDashAcrtivado?))
    (if (not (AI|Components|NavMovement|IsFalling (Variables|Character|GetCharacterMovement)))
      (if (not (Variables|Default|GetEstaAtacando))
        (Variables|Default|SetEstaAtacando true)
        (Pawn|Components|CharacterMovement|DisableMovement (Variables|Character|GetCharacterMovement))
        (Animation|Montage|PlayMontage (Variables|Character|GetMesh) (Utilities|Select :Index (Variables|Default|GetCantidadAtaques) :Option%200 "/Game/Characters/mixamo/animaciones/combate/AtaqueMele.AtaqueMele" :Option%201 "/Game/Characters/mixamo/animaciones/combate/Boxing_Montage.Boxing_Montage" :Option%202 "/Game/Characters/mixamo/animaciones/combate/Martelo_2_Montage.Martelo_2_Montage")
          (:then
            (Math|Integer|IncrementInt (Variables|Default|GetCantidadAtaques)
              (:%20%20
                (if (and (>= (Variables|/Game/componente/BP_ComponenteExperiencia.BP_ComponenteExperiencia_C|GetLevelPlayer (Variables|Default|GetBP_ComponenteExperiencia)) 3) (== (Variables|Default|GetCantidadAtaques) 4))
                  (Animation|Montage|PlayMontage (Variables|Character|GetMesh) "/Game/Characters/mixamo/animaciones/combate/Hurricane_Kick_Montage.Hurricane_Kick_Montage"
                    (:then
                      (Pawn|Components|CharacterMovement|SetMovementMode (Variables|Character|GetCharacterMovement) "MOVE_Walking" 0 :!label _label))
                    (:OnCompleted
                      (Variables|Default|SetCantidadAtaques 0 :!label _label_2))
                    (:OnBlendOut
                      (goto _label))
                    (:OnInterrupted
                      (Utilities|FlowControl|RetriggerableDelay 2.0)
                      (Variables|Default|SetEstaAtacando false)
                      (goto _label_2)))))))
          (:OnCompleted
            (Variables|Default|SetCantidadAtaques 0 :!label _label_3))
          (:OnBlendOut
            (Pawn|Components|CharacterMovement|SetMovementMode (Variables|Character|GetCharacterMovement) "MOVE_Walking" 0))
          (:OnInterrupted
            (Utilities|FlowControl|RetriggerableDelay 2.0)
            (Variables|Default|SetEstaAtacando false)
            (goto _label_3)))))))

(event Input|EnhancedActionEvents|EnhancedInputActionIA_Interactuar
  (params (ActionValue :type Boolean) (ElapsedSeconds :type Float%20%28double-precision%29) (TriggeredSeconds :type Float%20%28double-precision%29) (InputAction :type Input%20Action%20Object%20Reference :default "/Game/imputs/IA_Interactuar.IA_Interactuar"))
  ;[0.15 0.15 0.15 0.5] Interactuar
  (Utilities|FlowControl|Sequence
    (:then_0
      (Class|BPIInteractuar|Interactuar(Message) (Utilities|Array|Get(acopy) (Collision|GetOverlappingActors "/Game/pickups/actores/BP_MasterPickupPrueba.BP_MasterPickupPrueba_C" :!class /Script/Engine.Actor)) self))
    (:then_1
      (CallFunction|InteractTrace)
      (bind _lookatactor (Variables|Default|GetLookAtActor)
        (:then
          (bind _objetiveid (Class|BPIInteractionQuest|Interactwith(Message) _lookatactor))
          (Default|CallOnObjetiveID _objetiveid 1))
        (:else)))))

(event Input|EnhancedActionEvents|EnhancedInputActionIA_Menu
  (params (ActionValue :type Boolean) (ElapsedSeconds :type Float%20%28double-precision%29) (TriggeredSeconds :type Float%20%28double-precision%29) (InputAction :type Input%20Action%20Object%20Reference :default "/Game/imputs/IA_Menu.IA_Menu")))

(event Input|EnhancedActionEvents|EnhancedInputActionIA_Disparo
  (params (ActionValue :type Boolean) (ElapsedSeconds :type Float%20%28double-precision%29) (TriggeredSeconds :type Float%20%28double-precision%29) (InputAction :type Input%20Action%20Object%20Reference :default "/Game/imputs/IA_Disparo.IA_Disparo"))
  (bind _returnvalue (Transformation|GetActorLocation))
  (bind _daño_disparo (Variables|Default|GetDaño%20Disparo))
  ;[0.15 0.15 0.15 0.5] ataque distancia
  (:Started
    (if (not (Variables|Default|GetDashAcrtivado?))
      (if (not (Variables|Default|GetEstaAtacando))
        (Collision|LineTraceForObjects _returnvalue (+ _returnvalue (* (Transformation|GetActorForwardVector) (Variables|Default|GetAlcanceDisparo))) (Utilities|Array|MakeArray "ObjectTypeQuery1" "ObjectTypeQuery2" "ObjectTypeQuery8") false 0 "None")
        (Pawn|Components|CharacterMovement|DisableMovement (Variables|Character|GetCharacterMovement))
        (Animation|Montage|PlayMontage (Variables|Character|GetMesh) "/Game/Characters/mixamo/animaciones/disparo/Shooting_Montage.Shooting_Montage"
          (:OnBlendOut
            (Utilities|FlowControl|Delay 0.5 :!label _label)
            (Pawn|Components|CharacterMovement|SetMovementMode (Variables|Character|GetCharacterMovement) "MOVE_Walking" 0)
            (Development|PrintString (Utilities|String|ToString(Float) _daño_disparo)))
          (:OnInterrupted
            (Utilities|FlowControl|RetriggerableDelay 2.0))
          (:OnNotifyBegin
            (Game|SpawnActorfromClass "/Game/quest/actores/BP_ProyectilDistancia.BP_ProyectilDistancia_C" (Transformation|GetWorldTransform (Variables|Default|GetArrow1)) "AdjustIfPossibleButAlwaysSpawn" "MultiplyWithRoot" 0 _daño_disparo 0)
            (goto _label)))))))

(event EventBeginPlay
  (bind _bp_componentevida (Variables|Default|GetBP_ComponenteVida))
  (bind _bp_componenteexperiencia (Variables|Default|GetBP_ComponenteExperiencia))
  (bind _asplayer_controller (Utilities|Casting|CastToPlayerController (Pawn|GetController))
    (:then
      (Input|AddMappingContext (PlayerController|LocalPlayerSubsystems|GetEnhancedInputLocalPlayerSubsystem _asplayer_controller) "/Game/imputs/IMC_Player.IMC_Player" 0 "(bIgnoreAllPressedKeysUntilRelease=True,bForceImmediately=False,bNotifyUserSettings=False)"))
    (:CastFailed
      _))
  (bind _returnvalue (UserInterface|CreateWidget "/Game/ui/WBP_ui.WBP_ui_C"))
  (UserInterface|Viewport|AddtoViewport _returnvalue 0)
  (CallFunction|ActualizarUi _returnvalue)
  (EventDispatchers|BindEventtoSaludIni _bp_componentevida (delegate Custom|salud%20inicial))
  (EventDispatchers|BindEventtoRecibiDano _bp_componentevida (delegate Custom|Dano%20recibido))
  (EventDispatchers|BindEventtoCuracion _bp_componentevida (delegate Custom|CuracionRecibida))
  (EventDispatchers|BindEventtoXPAlIniciar _bp_componenteexperiencia (delegate Custom|ExperienciaAlEmpezar))
  (EventDispatchers|BindEventtoSuboExperiencia _bp_componenteexperiencia (delegate Custom|SumoExperiencia))
  (EventDispatchers|BindEventtoLevIni _bp_componenteexperiencia (delegate Custom|levelinicial))
  (EventDispatchers|BindEventtoSuboNivel _bp_componenteexperiencia (delegate Custom|SumoLevel)))

(event Collision|EventActorBeginOverlap
  (params (OtherActor :type Actor%20Object%20Reference)))

(event EventDanoesfera
  (params (dano :type Float%20%28double-precision%29))
  ;[0.15 0.15 0.15 0.5] Recibir Daño
  (Default|DañoAlJugar (Variables|Default|GetBP_ComponenteVida) dano))

(event EventRealizarDanio
  (params (danio :type Float%20%28single-precision%29))
  ;[0.15 0.15 0.15 0.5] Recibir Daño
  (Default|DañoAlJugar (Variables|Default|GetBP_ComponenteVida) danio))

(event EventObtenerExperiencia
  (params (Experiencia :type Float%20%28double-precision%29))
  ;[0.15 0.15 0.15 0.5] Experiencia
  (Default|IncrementarExperiencia (Variables|Default|GetBP_ComponenteExperiencia) Experiencia))

(event EventOnLanded
  (params (Hit :type Hit%20Result%20Structure%20%28by%20ref%29))
  ;[0.15 0.15 0.15 0.5] salto
)

(event EventOnJumped
  ;[0.15 0.15 0.15 0.5] salto
)

(event EventTick
  (params (DeltaSeconds :type Float%20%28single-precision%29)))

(event Input|KeyboardEvents|DebugKeyT
  (params (Key :type Key%20Structure) (ActionValue :type Input%20Action%20Value%20Structure))
  (:Pressed
    (bind _returnvalue (UserInterface|CreateWidget "/Game/ui/questUI/WBP_VentanaMisiones.WBP_VentanaMisiones_C"))
    (UserInterface|Viewport|AddtoViewport _returnvalue 0)))

(event Input|KeyboardEvents|DebugKeyM
  (params (Key :type Key%20Structure) (ActionValue :type Input%20Action%20Value%20Structure))
  (bind _returnvalue (Game|GetPlayerController 0))
  ;[0.15 0.15 0.15 0.5] menu pausa debug
  (:Pressed
    (if (Utilities|IsValid (Variables|Default|GetPausaRef))
      (Development|PrintString "true")
      (Widget|RemovefromParent (Variables|Default|GetPausaRef))
      (Game|SetGamePaused true)
      (Variables|/Script/Engine.PlayerController|SetbShowMouseCursor _returnvalue false)
      (Variables|Default|SetPausaRef 0)
      (else
        (Development|PrintString "false")
        (bind _returnvalue_2 (UserInterface|CreateWidget "/Game/ui/WBP_MenuPausa.WBP_MenuPausa_C"))
        (bind _output_get (Variables|Default|SetPausaRef _returnvalue_2))
        (UserInterface|Viewport|AddtoViewport _output_get 0)
        (Game|SetGamePaused true)
        (Variables|/Script/Engine.PlayerController|SetbShowMouseCursor _returnvalue true)))))

(event Input|KeyboardEvents|DebugKeyP
  (params (Key :type Key%20Structure) (ActionValue :type Input%20Action%20Value%20Structure)))

(fn ConstructionScript)

(fn AddController
  (bind _asplayer_controller (Utilities|Casting|CastToPlayerController (Pawn|GetController)))
  (Input|AddMappingContext (PlayerController|LocalPlayerSubsystems|GetEnhancedInputLocalPlayerSubsystem _asplayer_controller) "/Game/imputs/IMC_Player.IMC_Player" 0 "(bIgnoreAllPressedKeysUntilRelease=True,bForceImmediately=False,bNotifyUserSettings=False)"))

(fn ActualizarUi
  (params (ui :type WBP%20Ui%20Object%20Reference))
  (bind _bp_componenteexperiencia (Variables|Default|GetBP_ComponenteExperiencia))
  (bind _bp_componentevida (Variables|Default|GetBP_ComponenteVida))
  (bind _output_get (Variables|Default|Setui ui))
  (Progress|SetPercent (Variables|/Game/ui/WBP_ui.WBP_ui_C|GetProgressBar_35 _output_get) (/ (Variables|/Game/componente/BP_ComponenteVida.BP_ComponenteVida_C|GetVida _bp_componentevida) (Variables|/Game/componente/BP_ComponenteVida.BP_ComponenteVida_C|GetVida%20max _bp_componentevida)))
  (Progress|SetPercent (Variables|/Game/ui/WBP_ui.WBP_ui_C|GetProgressBarEXP _output_get) (/ (Variables|/Game/componente/BP_ComponenteExperiencia.BP_ComponenteExperiencia_C|GetXP _bp_componenteexperiencia) (Variables|/Game/componente/BP_ComponenteExperiencia.BP_ComponenteExperiencia_C|GetMax%20XP _bp_componenteexperiencia))))

(fn InventarioUI
  (bind _returnvalue (UserInterface|CreateWidget "/Game/ui/WBP_Inventario.WBP_Inventario_C"))
  (bind _output_get (Variables|Default|SetInventario _returnvalue))
  (UserInterface|Viewport|AddtoViewport _output_get 0)
  (Default|CargarInventario _output_get (Variables|Default|GetBP_ComponenteInventario))
  (bind _output_get_2 (Variables|/Game/componente/BP_ComponenteInventario.BP_ComponenteInventario_C|SetInventarioWidget (Variables|Default|GetBP_ComponenteInventario) (Variables|Default|GetInventario)))
  (Widget|SetVisibility _output_get_2 "Hidden"))

(fn HitDetect
  (bind _mesh (Variables|Character|GetMesh))
  (bind _cantidadataques (Variables|Default|GetCantidadAtaques))
  (bind _returnvalue (Utilities|Select :Index _cantidadataques :Option%200 "None" :Option%201 "LeftHand" :Option%202 "RightLeg" :Option%203 "RightLeg" :Option%204 "LeftFoot"))
  (bind _returnvalue_2 (Transformation|GetSocketLocation _mesh _returnvalue))
  (bind _outhits (Collision|MultiSphereTraceForObjects _returnvalue_2 _returnvalue_2 5e+01 (Utilities|Array|MakeArray "ObjectTypeQuery8") false 0 "ForDuration"))
  (bind _array_element (Utilities|Array|ForEachLoopwithBreak _outhits)
    (:LoopBody
      (if (Utilities|DoesObjectImplementInterface (.HitActor (Collision|BreakHitResult _array_element)) "/Game/interfase/BPI_AtaqueMele.BPI_AtaqueMele_C")
        (Class|BPIAtaqueMele|GolpeVampiro(Message) (.HitActor (Collision|BreakHitResult _array_element)) 3e+01)))))

(fn CheckeoSalto
  (if (Variables|Default|GetPrimerSaltoHecho)
    (Variables|Default|SetPrimerSaltoHecho false)
    (Variables|Default|SetPuedoSaltar? false)
    (else
      (Variables|Default|SetPrimerSaltoHecho true))))

(fn InteractTrace
  (bind _returnvalue (Transformation|GetActorLocation))
  (bind (_outhit _returnvalue_2) (Collision|SphereTraceForObjects _returnvalue _returnvalue 1e+02 (Utilities|Array|MakeArray "ObjectTypeQuery3") false 0 "None"))
  (if _returnvalue_2
    (if (Utilities|DoesObjectImplementInterface (.HitActor (Collision|BreakHitResult _outhit)) "/Game/interfase/BPI_InteractionQuest.BPI_InteractionQuest_C")
      (bind _output_get (Variables|Default|SetLookAtActor (.HitActor (Collision|BreakHitResult _outhit))))
      (Class|BPIInteractionQuest|Lookat(Message) _output_get)
      (else
        (Variables|Default|SetLookAtActor 0)))
    (else
      (Variables|Default|SetLookAtActor 0))))