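; BP_EnemyBase is an enemy base actor with health and a viewport health bar widget.
; BPComponenteVida events update the bar, though the healing handler passes zeros.
; Sphere overlaps with BP_Character call MostrarBarraenemigo(true) on both enter and exit, despite the exit log saying hide.
; GolpeVampiro subtracts damage directly, refreshes the bar with a hardcoded maximum, and destroys the actor after a check that subtracts damage again.
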(event OnComponentBeginOverlap(Sphere)
  (params (OverlappedComponent :type Primitive%20Component%20Object%20Reference) (OtherActor :type Actor%20Object%20Reference) (OtherComp :type Primitive%20Component%20Object%20Reference) (OtherBodyIndex :type Integer) (bFromSweep :type Boolean) (SweepResult :type Hit%20Result%20Structure%20%28by%20ref%29))
  (bind _barravidaenemigo (Variables|Default|Getbarravidaenemigo))
  (Utilities|Casting|CastToBP_Character OtherActor)
  (Utilities|IsValid _barravidaenemigo
    (:Is%20Valid
      (Default|MostrarBarraenemigo _barravidaenemigo true)
      (Development|PrintString "entro mostrar barra"))))

(event OnComponentEndOverlap(Sphere)
  (params (OverlappedComponent :type Primitive%20Component%20Object%20Reference) (OtherActor :type Actor%20Object%20Reference) (OtherComp :type Primitive%20Component%20Object%20Reference) (OtherBodyIndex :type Integer))
  (bind _barravidaenemigo (Variables|Default|Getbarravidaenemigo))
  (Utilities|Casting|CastToBP_Character OtherActor)
  (Utilities|IsValid _barravidaenemigo
    (:Is%20Valid
      (Default|MostrarBarraenemigo _barravidaenemigo true)
      (Development|PrintString "salio esconderr barra"))))

(event Custom|SaludInicialEnemigo
  (params (Vida :type Float%20%28double-precision%29) (Vida%20max :type Float%20%28double-precision%29))
  (Default|ActualizarVidaEnemigo (Variables|Default|Getbarravidaenemigo) Vida Vida%20max))

(event Custom|EnemigoRecibioDano
  (params (Vida :type Float%20%28double-precision%29) (Vida%20max :type Float%20%28double-precision%29))
  (Default|ActualizarVidaEnemigo (Variables|Default|Getbarravidaenemigo) Vida Vida%20max))

(event Custom|EnemigoCurandose
  (params (Vida :type Float%20%28double-precision%29) (VidaMax :type Float%20%28double-precision%29))
  (Default|ActualizarVidaEnemigo (Variables|Default|Getbarravidaenemigo) 0.0 0.0))

(event EventBeginPlay
  (bind _bp_componentevida (Variables|Default|GetBP_ComponenteVida))
  (bind _returnvalue (UserInterface|CreateWidget "/Game/ui/BarraVidaEnemigo/WBP_BarraVidaEnemigo.WBP_BarraVidaEnemigo_C" (Game|GetPlayerController 0)))
  (bind _output_get (Variables|Default|Setbarravidaenemigo _returnvalue))
  (UserInterface|Viewport|AddtoViewport _output_get 0)
  (CallFunction|ActuiEnemigo _output_get)
  (EventDispatchers|BindEventtoSaludIni _bp_componentevida (delegate Custom|SaludInicialEnemigo))
  (EventDispatchers|BindEventtoRecibiDano _bp_componentevida (delegate Custom|EnemigoRecibioDano))
  (EventDispatchers|BindEventtoCuracion _bp_componentevida (delegate Custom|EnemigoCurandose)))

(event Collision|EventActorBeginOverlap
  (params (OtherActor :type Actor%20Object%20Reference)))

(event EventTick
  (params (DeltaSeconds :type Float%20%28single-precision%29)))

(event EventGolpeVampiro
  (params (daño :type Float%20%28double-precision%29))
  (bind _bp_componentevida (Variables|Default|GetBP_ComponenteVida))
  (bind _output_get (Variables|/Game/componente/BP_ComponenteVida.BP_ComponenteVida_C|SetVida _bp_componentevida (- (Variables|/Game/componente/BP_ComponenteVida.BP_ComponenteVida_C|GetVida _bp_componentevida) daño)))
  (CallFunction|EnemigoRecibioDano _output_get 1e+02)
  (if (<= (- (Variables|/Game/componente/BP_ComponenteVida.BP_ComponenteVida_C|GetVida _bp_componentevida) daño) 0.0)
    (Actor|DestroyActor)))

(fn ConstructionScript)

(fn ActuiEnemigo
  (params (barravidaenemigo :type WBP%20Barra%20Vida%20Enemigo%20Object%20Reference))
  (bind _bp_componentevida (Variables|Default|GetBP_ComponenteVida))
  (bind _output_get (Variables|Default|Setbarravidaenemigo barravidaenemigo))
  (Progress|SetPercent (Variables|/Game/ui/BarraVidaEnemigo/WBP_BarraVidaEnemigo.WBP_BarraVidaEnemigo_C|GetProgressBar_vidaenemigo _output_get) (/ (Variables|/Game/componente/BP_ComponenteVida.BP_ComponenteVida_C|GetVida _bp_componentevida) (Variables|/Game/componente/BP_ComponenteVida.BP_ComponenteVida_C|GetVida%20max _bp_componentevida))))