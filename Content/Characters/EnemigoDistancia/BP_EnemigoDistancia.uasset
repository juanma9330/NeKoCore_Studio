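; BP_EnemigoDistancia is a ranged enemy, referred to as Monja, that fires BP_Proyectil at the player.
; BeginPlay stores the player character as Target, which AtaqueDistancia passes to the spawned projectile with speed and damage.
; DisparoMonja is a separate shot taking an explicit objective, using a hardcoded speed and always spawning.
; Initial-health and damage events update its widget health bar from Vida over VidaMax, using a reference cached by the initial event.
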(event EventBeginPlay
  (|CallParentFunction)
  (CallFunction|SetTarget (CallFunction|GetMyPlayerCharacter)))

(event Collision|EventActorBeginOverlap
  (params (OtherActor :type Actor%20Object%20Reference))
  (|CallParentFunction OtherActor) ; This node is disabled and will not be called.\nDrag off pins to build functionality.
)

(event EventTick
  (params (DeltaSeconds :type Float%20%28single-precision%29))
  (|CallParentFunction DeltaSeconds))

(event EventSaludInicialEnemigo
  (params (Vida :type Float%20%28double-precision%29) (Vida%20max :type Float%20%28double-precision%29))
  (bind _aswbp_barra_vida_enemigo (Utilities|Casting|CastToWBP_BarraVidaEnemigo (UserInterface|GetWidget (Variables|Default|GetWidget))))
  (Variables|Default|SetAs%20WBP%20Barra%20Vida%20Enemigo_0 _aswbp_barra_vida_enemigo)
  (CallFunction|ActualizarVidaInicialMonja Vida Vida%20max))

(event EventAtaqueDistancia
  (Game|SpawnActorfromClass "/Game/Characters/EnemigoDistancia/BP_Proyectil.BP_Proyectil_C" (Transformation|GetActorTransform) "Undefined" "MultiplyWithRoot" 0 (Variables|Default|GetVelocidad%20Proyectil) (Variables|Default|GetDaño%20Proyectil) (Variables|Default|GetTarget) 0))

(event EventEnemigoRecibioDano
  (params (Vida :type Float%20%28double-precision%29) (Vida%20max :type Float%20%28double-precision%29))
  (CallFunction|ActualizarVidaInicialMonja Vida Vida%20max))

(fn ConstructionScript
  (|CallParentFunction))

(fn DisparoMonja
  (params (objetivo :type BP%20Character%20Object%20Reference))
  (Game|SpawnActorfromClass "/Game/Characters/EnemigoDistancia/BP_Proyectil.BP_Proyectil_C" (Transformation|GetActorTransform) "AlwaysSpawn" "MultiplyWithRoot" 0 1e+01 (Variables|Default|GetDaño%20Proyectil) objetivo 0))

(fn ActualizarVidaInicialMonja
  (params (vida :type Float%20%28double-precision%29) (Vida%20Max :type Float%20%28double-precision%29))
  (Progress|SetPercent (Variables|/Game/ui/BarraVidaEnemigo/WBP_BarraVidaEnemigo.WBP_BarraVidaEnemigo_C|GetProgressBar_vidaenemigo (Variables|Default|GetAs%20WBP%20Barra%20Vida%20Enemigo_0)) (/ vida Vida%20Max)))

(fn SetTarget
  (params (Target :type BP%20Character%20Object%20Reference))
  (Variables|Default|SetTarget Target))