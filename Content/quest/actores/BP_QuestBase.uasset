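; Base quest actor that tracks objective progress for the current stage of a quest.
; On BeginPlay it loads the stage from the quest data table, zeroes a progress map and binds to the player's objective-ID event.
; OnObjetiveIDHeard updates counts; reaching a required quantity shows a notification, grants bonus XP and rechecks completion.
; The startup inventory query's result is unused, and the stage XP reward is disconnected.
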(event EventBeginPlay
  (CallFunction|GetQuestDeatails)
  (EventDispatchers|BindEventtoOnObjetiveID (CallFunction|GetMyPlayerCharacter) (EventDispatchers|CreateEvent :!event OnObjetiveIDHeard))
  (for _array_element (.Objetives (Utilities|Struct|BreakS_StageDetails (Variables|Default|GetCurrentStageDetails)))
    (if (Utilities|Enum|Equal(Enum) (.Type (Utilities|Struct|BreakS_ObjetiveDetails _array_element)) "NewEnumerator3")
      (bind _value (Default|QueryInventory (Variables|/Game/Characters/BP_Character.BP_Character_C|GetBP_ComponenteInventario (CallFunction|GetMyPlayerCharacter)) (Utilities|String|StringToName (.ObjetiveID (Utilities|Struct|BreakS_ObjetiveDetails _array_element)))))))
  (Utilities|FlowControl|Delay 1.0)
  (bind _return (CallFunction|MisionCompletada))
  (Variables|Default|SetIsCompleted _return))

(event Collision|EventActorBeginOverlap
  (params (OtherActor :type Actor%20Object%20Reference)))

(event EventTick
  (params (DeltaSeconds :type Float%20%28single-precision%29)))

(fn ConstructionScript)

(fn OnObjetiveIDHeard
  (params (ObjetiveID :type String) (Value :type Integer))
  (bind _currentobjetiveprogress (Variables|Default|GetCurrentObjetiveProgress))
  (bind (_value _returnvalue) (Utilities|Map|Find _currentobjetiveprogress ObjetiveID))
  (if (> (Class|KismetMathLibrary|SignOfInteger Value) 0)
    (if _returnvalue
      (if (< _value (.Quanty (Utilities|Struct|BreakS_ObjetiveDetails (CallFunction|GetObjetiveDatabyID ObjetiveID))))
        (Utilities|Map|Add (Variables|Default|GetCurrentObjetiveProgress) ObjetiveID (+ _value Value))
        (CallFunction|ObjetivoCompletado ObjetiveID)
        (CallFunction|MisionCompletada)
        (return))
      (else
        (return)))
    (else
      (Utilities|Map|Add (Variables|Default|GetCurrentObjetiveProgress) ObjetiveID (+ (.Value (Utilities|Map|Find (Variables|Default|GetCurrentObjetiveProgress) ObjetiveID)) Value))
      (return))))

(fn GetQuestDeatails
  (bind _returnvalue (Utilities|GetDataTableRow "/Game/quest/Data_Quest.Data_Quest" (Variables|Default|GetQuestID))
    (:then
      (bind _output_get (Variables|Default|SetQuestDetails _returnvalue))
      (bind _output_get_2 (Variables|Default|SetCurrentStageDetails (Utilities|Array|Get(acopy) (.Stages (Utilities|Struct|BreakS_MisionDetalles _output_get)) (Variables|Default|GetCurrentStage))))
      (Utilities|Map|Clear (Variables|Default|GetCurrentObjetiveProgress))
      (for _array_element (.Objetives (Utilities|Struct|BreakS_StageDetails _output_get_2))
        (Utilities|Map|Add (Variables|Default|GetCurrentObjetiveProgress) (.ObjetiveID (Utilities|Struct|BreakS_ObjetiveDetails _array_element)) 0)))))

(fn GetObjetiveDatabyID
  (params (ObjetiveID :type String))
  (for _array_element (.Objetives (Utilities|Struct|BreakS_StageDetails (Variables|Default|GetCurrentStageDetails)))
    (if (Utilities|Enum|Equal(Enum) (.ObjetiveID (Utilities|Struct|BreakS_ObjetiveDetails _array_element)) ObjetiveID)
      (return _array_element))))

(fn ObjetivoCompletado
  (params (ObjetiveID :type String))
  (bind _array_element (CallFunction|GetObjetiveDatabyID ObjetiveID))
  (bind (_objetivename _description _type _objetiveid _quanty _isoptional _bonusxp) (Utilities|Struct|BreakS_ObjetiveDetails _array_element))
  (if (>= (.Value (Utilities|Map|Find (Variables|Default|GetCurrentObjetiveProgress) ObjetiveID)) _quanty)
    (bind _returnvalue (UserInterface|CreateWidget "/Game/ui/questUI/WBP_NotificaciónMision.WBP_NotificaciónMision_C" 0 _description))
    (UserInterface|Viewport|AddtoViewport _returnvalue 0)
    (bind _return (CallFunction|MisionCompletada))
    (Variables|Default|SetIsCompleted _return)
    (Class|BPIExperiencia|ObtenerExperiencia(Message) (Game|GetPlayerCharacter 0) _bonusxp)))

(fn MisionCompletada
  (for _array_element (.Objetives (Utilities|Struct|BreakS_StageDetails (Variables|Default|GetCurrentStageDetails)))
    (if (not (>= (.Value (Utilities|Map|Find (Variables|Default|GetCurrentObjetiveProgress) (.ObjetiveID (Utilities|Struct|BreakS_ObjetiveDetails _array_element)))) (.Quanty (Utilities|Struct|BreakS_ObjetiveDetails (CallFunction|GetObjetiveDatabyID (.ObjetiveID (Utilities|Struct|BreakS_ObjetiveDetails _array_element)))))))
      (bind _output_get (LocalVariables|SetLocal_AllComplete false))
      (return _output_get)))
  (return (LocalVariables|GetLocal_AllComplete)))