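; Quest giver component that offers a quest and shows its reward screen when its owner is interacted with.
; InteractWith asks the player's BPComponenteMisiones whether the QuestData row is active, opening WBP_MisionesNPC if it is not.
; For active quests it always prints a not-completed message, then opens WBP_Recompensa if the quest actor is completed.
; Both widgets receive data table rows, though the reward lookup uses Data_Quest directly instead of QuestData's table.
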(event EventBeginPlay)

(event EventTick
  (params (DeltaSeconds :type Float%20%28single-precision%29)))

(fn DsiplayQuest
  (bind _questdata (Variables|Default|GetQuestData))
  (bind _returnvalue (Utilities|GetDataTableRow (.datatable _questdata) (.rowname _questdata))
    (:then
      (bind _returnvalue_2 (UserInterface|CreateWidget "/Game/ui/questUI/WBP_MisionesNPC.WBP_MisionesNPC_C" 0 _returnvalue (.rowname _questdata) 0))
      (UserInterface|Viewport|AddtoViewport _returnvalue_2 0))))

(fn DisplayRecompensa
  (bind _questdata (Variables|Default|GetQuestData))
  (bind _returnvalue (Utilities|GetDataTableRow "/Game/quest/Data_Quest.Data_Quest" (.rowname _questdata))
    (:then
      (bind _returnvalue_2 (UserInterface|CreateWidget "/Game/ui/questUI/WBP_Recompensa.WBP_Recompensa_C" 0 _returnvalue (.rowname _questdata) 0))
      (UserInterface|Viewport|AddtoViewport _returnvalue_2 0))))

(fn Interactwith
  (bind _returnvalue (Components|GetOwner))
  (bind _returnvalue_2 (Utilities|GetDisplayName _returnvalue))
  (if (not (Default|QueryActiveQuest (Variables|/Game/Characters/BP_Character.BP_Character_C|GetBP_ComponenteMisiones (CallFunction|GetMyPlayerCharacter)) (.rowname (Variables|Default|GetQuestData))))
    (CallFunction|DsiplayQuest)
    (return _returnvalue_2)
    (else
      (bind _array_element (Default|GetQuestActor (Variables|/Game/Characters/BP_Character.BP_Character_C|GetBP_ComponenteMisiones (CallFunction|GetMyPlayerCharacter)) (.rowname (Variables|Default|GetQuestData))))
      (Development|PrintString "Todavia no completaste la mision")
      (if (Variables|/Game/quest/actores/BP_QuestBase.BP_QuestBase_C|GetIsCompleted _array_element)
        (CallFunction|DisplayRecompensa)
        (return _returnvalue_2)))))