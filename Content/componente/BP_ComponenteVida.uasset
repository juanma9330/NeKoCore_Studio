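; BP_ComponenteVida is a health component that tracks current and maximum life for its owner.
; One tick after BeginPlay, it broadcasts the starting values through the SaludIni dispatcher.
; The Danoesfera event passes damage to DañoAlJugar, which subtracts it from Vida, clamped between zero and VidaMax, and broadcasts the result through the Daño dispatcher.
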(event EventBeginPlay
  (Utilities|FlowControl|DelayUntilNextTick)
  (CallFunction|SaludInicial))

(event EventTick
  (params (DeltaSeconds :type Float%20%28single-precision%29)))

(event EventDanoesfera
  (params (dano :type Float%20%28double-precision%29))
  (CallFunction|DañoAlJugar dano))

(fn SaludInicial
  (Default|CallSaludIni (Variables|Default|GetVida) (Variables|Default|GetVida%20max)))

(fn DañoAlJugar
  (params (dano :type Float%20%28double-precision%29))
  (bind _output_get (Variables|Default|SetVida (Math|Float|Clamp(Float) (- (Variables|Default|GetVida) dano) 0.0 (Variables|Default|GetVida%20max))))
  (Default|CallDaño _output_get (Variables|Default|GetVida%20max)))