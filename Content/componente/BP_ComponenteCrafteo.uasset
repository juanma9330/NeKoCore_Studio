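; Crafting component that toggles the crafting/inventory menu and tracks which recipes are unlocked.
; CalculoInicial reads the row names of a given DataTable, unlocks rows with no level requirement or one met by CurrentLevel, blocking-loads item classes, and prints the result.
; The IA_Inventario action lazily creates WBP_Inventario, switches input mode and cursor, and passes DataCrafteo and the unlocked names to the widget on opening.
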(event Custom|CalculoInicial
  (params (LaDatatableenuso :type Data%20Table%20Object%20Reference))
  (Variables|Default|SetLa%20Datatableenuso LaDatatableenuso)
  (bind _outrownames (DataTable|GetDataTableRowNames (Variables|Default|GetLa%20Datatableenuso)))
  (Variables|Default|SetTodos%20los%20itemsCafteables _outrownames)
  (CallFunction|CalculateUnlockItems)
  (CallFunction|PrintUnlockedItem))

(event Input|EnhancedActionEvents|EnhancedInputActionIA_Inventario
  (params (ActionValue :type Boolean) (ElapsedSeconds :type Float%20%28double-precision%29) (TriggeredSeconds :type Float%20%28double-precision%29) (InputAction :type Input%20Action%20Object%20Reference :default "/Game/imputs/IA_Inventario.IA_Inventario"))
  (bind _returnvalue (Game|GetPlayerController 0))
  (bind _returnvalue_2 (Game|GetPlayerController 0))
  (:Completed
    (Utilities|IsValid (Variables|Default|GetMenuCrafteos)
      (:Is%20Valid
        (if (Widget|IsVisible (Variables|Default|GetMenuCrafteos))
          (Widget|SetVisibility (Variables|Default|GetMenuCrafteos) "Hidden")
          (Input|SetInputModeGameOnly _returnvalue_2 false)
          (Variables|/Script/Engine.PlayerController|SetbShowMouseCursor _returnvalue_2 false)
          (else
            (UserInterface|Viewport|AddtoViewport (Variables|Default|GetMenuCrafteos) 0 :!label _label)
            (Input|SetInputModeGameandUI _returnvalue (Variables|Default|GetMenuCrafteos) "DoNotLock" true false)
            (Variables|/Script/Engine.PlayerController|SetbShowMouseCursor _returnvalue true)
            (Default|ActualizacionMateriales (Variables|Default|GetMenuCrafteos) "/Game/Datatable/DataCrafteo.DataCrafteo" (Variables|Default|GetUnlockCrafteableItems))
            (Widget|SetVisibility (Variables|Default|GetMenuCrafteos) "Visible"))))
      (:Is%20Not%20Valid
        (bind _returnvalue_3 (UserInterface|CreateWidget "/Game/ui/WBP_Inventario.WBP_Inventario_C"))
        (Variables|Default|SetMenuCrafteos _returnvalue_3)
        (goto _label)))))

(event EventBeginPlay)

(event EventTick
  (params (DeltaSeconds :type Float%20%28single-precision%29)))

(fn CalculateUnlockItems
  (for _array_element (Variables|Default|GetTodos%20los%20itemsCafteables)
    (LocalVariables|SetCurrentArrayElements _array_element)
    (if (not (Utilities|Array|ContainsItem (Variables|Default|GetUnlockCrafteableItems) (LocalVariables|GetCurrentArrayElements)))
      (bind _out_row (CallFunction|Getnombresdecrafteables (LocalVariables|GetCurrentArrayElements)))
      (LocalVariables|SetCurrentitemrow _out_row)
      (if (Utilities|IsValidClass (Utilities|ResolveSoftReference (.ItemCrafteable1 (Utilities|Struct|BreakS_Crafteo (LocalVariables|GetCurrentitemrow)))))
        _
        (else
          (Utilities|LoadClassAssetBlocking (Utilities|Struct|BreakS_Crafteo (LocalVariables|GetCurrentitemrow)))))
      (if (== (Utilities|Struct|BreakS_Crafteo (LocalVariables|GetCurrentitemrow)) 0)
        (Utilities|Array|Add (Variables|Default|GetUnlockCrafteableItems) (LocalVariables|GetCurrentArrayElements) :!label _label)
        (elif (>= (Variables|Default|GetCurrentLevel) (Utilities|Struct|BreakS_Crafteo (LocalVariables|GetCurrentitemrow)))
          (goto _label))))))

(fn Getnombresdecrafteables
  (params (rowname :type Name))
  (bind _la_datatableenuso (Variables|Default|GetLa%20Datatableenuso))
  (bind _returnvalue (Class|DataTableFunctionLibrary|DoesDataTableRowExist _la_datatableenuso rowname))
  (if _returnvalue
    (bind _returnvalue_2 (Utilities|GetDataTableRow _la_datatableenuso rowname)
      (:then
        (return _returnvalue_2)))))

(fn PrintUnlockedItem
  (for _array_element (Variables|Default|GetUnlockCrafteableItems)
    (Development|PrintString (Utilities|String|ToString(Name) _array_element))))