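; Inventory component that gives the player an eight-slot item array shown in WBP_Inventario.
; Debug key O toggles the widget; R sphere-traces around the player for a BP_ItemInventario, stacks up to three or fills empty slots without breaking the loop.
; Merged stacks are written at the slot's quantity as index, not its loop index.
; A separate Content map tallies items and reports objective progress to BP_Character, alongside a simple Lista.
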(event EventBeginPlay
  (Utilities|FlowControl|DelayUntilNextTick)
  (bind _returnvalue (UserInterface|CreateWidget "/Game/ui/WBP_Inventario.WBP_Inventario_C"))
  (Variables|Default|SetWBP_Inventario _returnvalue)
  (Utilities|Array|Resize (Variables|Default|GetItems) 8)
  (Default|CargarInventario (Variables|Default|GetWBP_Inventario) self))

(event EventTick
  (params (DeltaSeconds :type Float%20%28single-precision%29)))

(event Input|KeyboardEvents|DebugKeyO
  (params (Key :type Key%20Structure :default "None") (ActionValue :type Input%20Action%20Value%20Structure))
  (bind _returnvalue (Game|GetPlayerController 0))
  (bind _returnvalue_2 (Game|GetPlayerController 0))
  (bind _wbp_inventario (Variables|Default|GetWBP_Inventario))
  (:Pressed
    (if (Widget|IsVisible (Variables|Default|GetWBP_Inventario))
      (Widget|RemovefromParent _wbp_inventario)
      (Variables|/Script/Engine.PlayerController|SetbShowMouseCursor _returnvalue_2 true)
      (Input|SetInputModeGameOnly _returnvalue_2 false)
      (else
        (Variables|/Script/Engine.PlayerController|SetbShowMouseCursor _returnvalue true)
        (Input|SetInputModeGameandUI _returnvalue 0 "DoNotLock" true false)
        (UserInterface|Viewport|AddtoViewport _wbp_inventario 0)))))

(event Input|KeyboardEvents|DebugKeyR
  (params (Key :type Key%20Structure :default "None") (ActionValue :type Input%20Action%20Value%20Structure))
  (bind _returnvalue (Game|GetPlayerCharacter 0))
  (bind _returnvalue_2 (Transformation|GetActorLocation _returnvalue))
  (:Pressed
    (bind _outhit (Collision|SphereTraceByChannel _returnvalue_2 _returnvalue_2 2e+02 "TraceTypeQuery1" false 0 "None"))
    (bind _asbp_item_inventario (Utilities|Casting|CastToBP_ItemInventario (.HitActor (Collision|BreakHitResult _outhit))))
    (for (_array_element _array_index) (Variables|Default|GetItems)
      (if (Math|Boolean|ANDBoolean (Utilities|Enum|Equal(Enum) (.nombre (Utilities|Struct|BreakS_Inventario _array_element)) (.nombre (Utilities|Struct|BreakS_Inventario (Variables|/Game/Actores/ModelosInventario/BP_ItemInventario.BP_ItemInventario_C|GetItemInventario _asbp_item_inventario)))) (.PuedoLlevarMasDeUno? (Utilities|Struct|BreakS_Inventario (Variables|/Game/Actores/ModelosInventario/BP_ItemInventario.BP_ItemInventario_C|GetItemInventario _asbp_item_inventario))) (<= (+ (.Cantidad (Utilities|Struct|BreakS_Inventario _array_element)) (.Cantidad (Utilities|Struct|BreakS_Inventario (Variables|/Game/Actores/ModelosInventario/BP_ItemInventario.BP_ItemInventario_C|GetItemInventario _asbp_item_inventario)))) 3))
        (Utilities|Array|SetArrayElem (Variables|Default|GetItems) (.Cantidad (Utilities|Struct|BreakS_Inventario _array_element)) (Utilities|Struct|MakeS_Inventario (.nombre (Variables|/Game/Actores/ModelosInventario/BP_ItemInventario.BP_ItemInventario_C|GetItemInventario _asbp_item_inventario)) (.puedollevarmasdeuno? (Variables|/Game/Actores/ModelosInventario/BP_ItemInventario.BP_ItemInventario_C|GetItemInventario _asbp_item_inventario)) (+ (.Cantidad (Utilities|Struct|BreakS_Inventario _array_element)) (.Cantidad (Utilities|Struct|BreakS_Inventario (Variables|/Game/Actores/ModelosInventario/BP_ItemInventario.BP_ItemInventario_C|GetItemInventario _asbp_item_inventario)))) (.miniatura (Variables|/Game/Actores/ModelosInventario/BP_ItemInventario.BP_ItemInventario_C|GetItemInventario _asbp_item_inventario)) (.mesh (Variables|/Game/Actores/ModelosInventario/BP_ItemInventario.BP_ItemInventario_C|GetItemInventario _asbp_item_inventario))))
        (Default|CargarInventario (Variables|Default|GetWBP_Inventario) self :!label _label)
        (Actor|DestroyActor _asbp_item_inventario)
        (elif (== (.Cantidad (Utilities|Struct|BreakS_Inventario _array_element)) 0)
          (Utilities|Array|SetArrayElem (Variables|Default|GetItems) _array_index (Variables|/Game/Actores/ModelosInventario/BP_ItemInventario.BP_ItemInventario_C|GetItemInventario _asbp_item_inventario))
          (goto _label))))))

(fn AddItemstoinventory
  (params (NewItem :type String%20%28by%20ref%29))
  (Utilities|Array|Add (Variables|Default|Getlista) NewItem)
  (Development|PrintString NewItem))

(fn AnadirAlInventario
  (params (item :type Name) (cantidad :type Integer))
  (Utilities|Map|Add (Variables|Default|GetContent) item (+ cantidad (.Value (Utilities|Map|Find (Variables|Default|GetContent) item))))
  (bind _asbp_character (Utilities|Casting|CastToBP_Character (Game|GetPlayerCharacter 0)))
  (Default|CallOnObjetiveID _asbp_character (Utilities|String|ToString(Name) item) cantidad))

(fn QueryInventory
  (params (item :type Name))
  (return (.Value (Utilities|Map|Find (Variables|Default|GetContent) item))))