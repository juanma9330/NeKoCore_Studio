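; Experience component that tracks XP and level for the actor that owns it.
; Adding XP past the current maximum raises the level by one, increases the next threshold by a fixed amount and resets XP to zero, discarding any overflow.
; Event dispatchers broadcast XP and level changes, plus the initial values one tick after BeginPlay.
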(event EventBeginPlay
  (Utilities|FlowControl|DelayUntilNextTick)
  (CallFunction|ExpInicial)
  (CallFunction|LevelInicial))

(event EventTick
  (params (DeltaSeconds :type Float%20%28single-precision%29)))

(fn IncrementarExperiencia
  (params (XP%20Añadida :type Float%20%28double-precision%29))
  (Variables|Default|SetXP (+ (Variables|Default|GetXP) XP%20Añadida))
  (Default|CallSuboExperiencia (Variables|Default|GetXP) (Variables|Default|GetMax%20XP))
  (if (> (Variables|Default|GetXP) (Variables|Default|GetMax%20XP))
    (CallFunction|IncrementarLevel 1 3.5e+02)))

(fn IncrementarLevel
  (params (AñadeLevel :type Integer) (Incrementar%20MaxExp :type Float%20%28double-precision%29))
  (Variables|Default|SetLevel (+ (Variables|Default|GetLevel) AñadeLevel))
  (Default|CallSuboNivel (Variables|Default|GetLevel))
  (Variables|Default|SetMax%20XP (+ (Variables|Default|GetMax%20XP) Incrementar%20MaxExp))
  (Variables|Default|SetXP 0.0))

(fn ExpInicial
  (Default|CallXPAlIniciar (Variables|Default|GetXP) (Variables|Default|GetMax%20XP)))

(fn LevelInicial
  (Default|CallLevIni (Variables|Default|GetLevel)))