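; BP_Character is the player character, with Enhanced Input movement and an on-screen health bar.
; BeginPlay adds the IMC_Player mapping context, creates the UI widget and sets its progress bar once from the ComponenteSalud health ratio.
; IA_Movimiento feeds movement input along fixed world X and Y axes, independent of camera or control rotation.
; The SaludInicial function is an empty stub.
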(event Input|EnhancedActionEvents|EnhancedInputActionIA_Movimiento
  (params (ActionValue :type Vector%202D%20Structure) (ElapsedSeconds :type Float%20%28double-precision%29) (TriggeredSeconds :type Float%20%28double-precision%29) (InputAction :type Input%20Action%20Object%20Reference :default "/Game/imputs/IA_Movimiento.IA_Movimiento"))
  (bind (_x _y) (Math|Vector2D|BreakVector2D ActionValue))
  (Pawn|Input|AddMovementInput "1.000000,0.000000,0.000000" _x false)
  (Pawn|Input|AddMovementInput "0.000000,1.000000,0.000000" _y false))

(event EventBeginPlay
  (bind _componentesalud (Variables|Default|GetComponenteSalud))
  (CallFunction|AddController)
  (bind _returnvalue (UserInterface|CreateWidget "/Game/ui/ui.ui_C"))
  (UserInterface|Viewport|AddtoViewport _returnvalue 0)
  (bind _output_get (Variables|Default|Setui _returnvalue))
  (Progress|SetPercent (Variables|/Game/ui/ui.ui_C|GetProgressBar_35 _output_get) (Math|Conversions|ToFloat(Integer) (/ (Variables|/Script/proyectoejercicio.ComponenteSalud|GetSalud _componentesalud) (Variables|/Script/proyectoejercicio.ComponenteSalud|GetSaludMax _componentesalud)))))

(event Collision|EventActorBeginOverlap
  (params (OtherActor :type Actor%20Object%20Reference)))

(event EventTick
  (params (DeltaSeconds :type Float%20%28single-precision%29)))

(fn ConstructionScript)

(fn AddController
  (bind _asplayer_controller (Utilities|Casting|CastToPlayerController (Pawn|GetController)))
  (Input|AddMappingContext (PlayerController|LocalPlayerSubsystems|GetEnhancedInputLocalPlayerSubsystem _asplayer_controller) "/Game/imputs/IMC_Player.IMC_Player" 0 "(bIgnoreAllPressedKeysUntilRelease=True,bForceImmediately=False,bNotifyUserSettings=False)"))

(fn SaludInicial
  (params (salud :type Float%20%28double-precision%29) (Salud%20max :type Float%20%28double-precision%29)))